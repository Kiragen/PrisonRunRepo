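; Player character Blueprint that maps input to walking, looking and jumping.
; Forward/back and strafe axes add movement along the forward and right vectors of the mesh's world rotation, rather than the control rotation.
; Yaw input turns the controller, while pitch rotates the camera component directly with no clamp in the graph.
; The jump action calls the built-in Jump on press, and the construction script is empty.
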(event Input|ActionEvents|InputActionJump
  (params (Key :type Key%20Structure))
  ;[1 1 1] Camera Controls & Jump
  (:Pressed
    (Character|Jump)))

(event Input|AxisEvents|InputAxisRight_Left
  (params (AxisValue :type Float%20%28single-precision%29))
  ;[1 1 1] Up Down Left Right movement
  (Pawn|Input|AddMovementInput (Math|Vector|GetRightVector (Transformation|GetWorldRotation (Variables|Character|GetMesh))) AxisValue false))

(event Input|AxisEvents|InputAxisUp_down
  (params (AxisValue :type Float%20%28single-precision%29))
  ;[1 1 1] Up Down Left Right movement
  (Pawn|Input|AddMovementInput (Math|Vector|GetForwardVector (Transformation|GetWorldRotation (Variables|Character|GetMesh))) AxisValue false))

(event Input|AxisEvents|InputAxisPitch
  (params (AxisValue :type Float%20%28single-precision%29))
  ;[1 1 1] Camera Controls & Jump
  (Transformation|AddRelativeRotation (Variables|Default|GetCamera) (Math|Rotator|MakeRotator 0.0 AxisValue 0.0) false false))

(event Input|AxisEvents|InputAxisYaw
  (params (AxisValue :type Float%20%28single-precision%29))
  ;[1 1 1] Camera Controls & Jump
  (Pawn|Input|AddControllerYawInput AxisValue))

(fn ConstructionScript)